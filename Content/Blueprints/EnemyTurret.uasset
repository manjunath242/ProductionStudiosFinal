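; Enemy turret that tracks the player pawn and fires from two barrels while the player is within attack range.
; Tick updates the range flag, which gates both aiming and firing.
; Aiming smoothly interpolates the gun toward a look-at rotation, with offset yaw, clamped roll and zero pitch.
; A Delay re-entered from Tick paces the spawning of Blueprint_Effect_Fire1 actors at both barrel sockets.
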(event `self.ReceiveTick`
  (params (DeltaSeconds :type "Float (single-precision)"))
  ;[1 1 1] game loop
  (set `self.DeltaTime` DeltaSeconds)
  (`self.UpdateRange`)
  (`self.Update Rotation`)
  (`self.Fire Weapon`))

(event `Update Rotation`
  ;[1 1 1] TurretRotation
  (if (`self.EnemyInRange`)
    (`SceneComponent.K2_SetWorldRotation` (`self.TurretGun`) (`KismetMathLibrary.RInterpTo` (`SceneComponent.K2_GetComponentRotation` (`self.TurretGun`)) (`KismetMathLibrary.MakeRotator` (`KismetMathLibrary.ClampAngle` (- (.roll (`KismetMathLibrary.FindLookAtRotation` (`SceneComponent.K2_GetComponentLocation` (`self.TurretGun`)) (`self.K2_GetActorLocation` (`GameplayStatics.GetPlayerPawn` 0)))) (`self.BarrelLength`)) -10.0 35.0) 0.0 (- (.yaw (`KismetMathLibrary.FindLookAtRotation` (`SceneComponent.K2_GetComponentLocation` (`self.TurretGun`)) (`self.K2_GetActorLocation` (`GameplayStatics.GetPlayerPawn` 0)))) 90.0)) (`self.DeltaTime`) (`self.RotationSpeed`)) false false)))

(event `Fire Weapon`
  (bind _turretgun (`self.TurretGun`))
  ;[1 1 1] BulletSpawning
  (if (`self.EnemyInRange`)
    (`KismetSystemLibrary.Delay` (`self.FireInterval`))
    (`|SpawnActorFromClass` "/Game/StarterContent/Blueprints/Blueprint_Effect_Fire1.Blueprint_Effect_Fire1_C" (`SceneComponent.GetSocketTransform` _turretgun "Barrel_1" "RTS_World") "Undefined" "OverrideRootScale")
    (`|SpawnActorFromClass` "/Game/StarterContent/Blueprints/Blueprint_Effect_Fire1.Blueprint_Effect_Fire1_C" (`SceneComponent.GetSocketTransform` _turretgun "Barrel_2" "RTS_World") "Undefined" "OverrideRootScale")))

(event `UpdateRange`
  ;[1 1 1] UpdateRange
  (if (<= (`self.GetDistanceTo` self (`GameplayStatics.GetPlayerPawn` 0)) (`self.AttackRange`))
    (set `self.EnemyInRange` true)
    (else
      (set `self.EnemyInRange` false))))

(fn `UserConstructionScript`)