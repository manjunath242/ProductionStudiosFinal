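; Rotating rock obstacle that destroys a BP_SpaceShip on collision and can itself be destroyed through health loss.
; The construction script applies a configurable mesh and RotatingMovement settings for rate, pivot and space.
; Any mesh hit spawns an explosion at the impact and plays a collapse sound at world origin, then destroys the hit actor if it is the ship.
; DecreaseHealth decrements Health and destroys the rock at zero.
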(event `DecreaseHealth`
  (bind _result (`/Engine/EditorBlueprintResources/StandardMacros.DecrementInt` (`self.Health`))
    (:`  `
      (if (<= _result 0)
        (`self.K2_DestroyActor`)))))

(event `self.StaticMeshComponent.OnComponentHit`
  (params (HitComponent :type "PrimitiveComponent Object Reference") (OtherActor :type "Actor Object Reference") (OtherComp :type "PrimitiveComponent Object Reference") (NormalImpulse :type "Vector Structure") (Hit :type "HitResult Structure (by ref)"))
  (bind (_bblockinghit _binitialoverlap _time _location _impactpoint _normal _impactnormal _physmat _hitactor) (`GameplayStatics.BreakHitResult` Hit))
  (`GameplayStatics.SpawnEmitterAtLocation` "/Game/StarterContent/Particles/P_Explosion.P_Explosion" _location)
  (`GameplayStatics.PlaySoundAtLocation` "/Game/StarterContent/Audio/Collapse01.Collapse01")
  (bind _asbp_space_ship (cast `/Game/Blueprints/BP_SpaceShip` _hitactor))
  (`self.K2_DestroyActor` _asbp_space_ship))

(fn `UserConstructionScript`
  (bind _rotatingmovement (`self.RotatingMovement`))
  (`StaticMeshComponent.SetStaticMesh` (`self.StaticMeshComponent`) (`self.Mesh`))
  (set `RotatingMovementComponent.RotationRate` (`self.Rotation Rate`) _rotatingmovement)
  (set `RotatingMovementComponent.PivotTranslation` (`self.Pivot Translation`) _rotatingmovement)
  (set `RotatingMovementComponent.bRotationInLocalSpace` (`self.Rotation in Local Space`) _rotatingmovement))