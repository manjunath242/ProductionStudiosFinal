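; Player-controlled physics spaceship with toggleable cockpit and external cameras and a hitscan weapon for shooting rocks.
; Axis inputs drive paired thruster components for roll, pitch and yaw, while engine input applies forward impulses to the mesh.
; Tick tints three cylinders' dynamic materials from grey to red-orange using summed velocity components.
; Left-click line-traces forward, spawns explosion effects even without a hit, and decreases health on Rock_84_Blueprint actors.
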(event `InputAction|ToggleCameraView`
  (params (Key :type "Key Structure" :default "AnyKey"))
  (bind _cockpitcamera (`self.CockpitCamera`))
  (bind _externalcamera (`self.ExternalCamera`))
  ;[1 1 1] Handles switching between ExternalCamera and CockpitCamera
  (:`Pressed`
    (`/Engine/EditorBlueprintResources/StandardMacros.FlipFlop`
      (:`A`
        (`ActorComponent.Activate` _cockpitcamera false)
        (`ActorComponent.Deactivate` _externalcamera))
      (:`B`
        (`ActorComponent.Deactivate` _cockpitcamera)
        (`ActorComponent.Activate` _externalcamera false)))))

(event `InputAxis|Roll`
  (params (AxisValue :type "Float (single-precision)"))
  (bind _leftwingrollthrust (`self.LeftWingRollThrust`))
  (bind _rightwingrollthrust (`self.RightWingRollThrust`))
  (bind _returnvalue (* AxisValue (`self.RollStrength`)))
  ;[1 1 1] Handles Roll
  (if (!= AxisValue 0.0)
    (set `PhysicsThrusterComponent.ThrustStrength` _returnvalue _leftwingrollthrust)
    (set `PhysicsThrusterComponent.ThrustStrength` _returnvalue _rightwingrollthrust)
    (`ActorComponent.Activate` _leftwingrollthrust false)
    (`ActorComponent.Activate` _rightwingrollthrust false)
    (else
      (`ActorComponent.Deactivate` (`self.LeftWingRollThrust`))
      (`ActorComponent.Deactivate` (`self.RightWingRollThrust`)))))

(event `InputAxis|Pitch`
  (params (AxisValue :type "Float (single-precision)"))
  (bind _nosepitchthrust (`self.NosePitchThrust`))
  (bind _tailpitchthrust (`self.TailPitchThrust`))
  (bind _returnvalue (* AxisValue (`self.PitchStrength`)))
  ;[1 1 1] Handles Pitch
  (if (!= 0.0 AxisValue)
    (set `PhysicsThrusterComponent.ThrustStrength` _returnvalue _nosepitchthrust)
    (set `PhysicsThrusterComponent.ThrustStrength` _returnvalue _tailpitchthrust)
    (`ActorComponent.Activate` _nosepitchthrust false)
    (`ActorComponent.Activate` _tailpitchthrust false)
    (else
      (`ActorComponent.Deactivate` (`self.NosePitchThrust`))
      (`ActorComponent.Deactivate` (`self.TailPitchThrust`)))))

(event `InputAxis|Yaw`
  (params (AxisValue :type "Float (single-precision)"))
  (bind _noseyawthrust (`self.NoseYawThrust`))
  (bind _tailyawthrust (`self.TailYawThrust`))
  (bind _returnvalue (* AxisValue (`self.YawStrength`)))
  ;[1 1 1] Handles Yaw
  (if (!= AxisValue 0.0)
    (set `PhysicsThrusterComponent.ThrustStrength` _returnvalue _noseyawthrust)
    (set `PhysicsThrusterComponent.ThrustStrength` _returnvalue _tailyawthrust)
    (`ActorComponent.Activate` _noseyawthrust false)
    (`ActorComponent.Activate` _tailyawthrust false)
    (else
      (`ActorComponent.Deactivate` (`self.NoseYawThrust`))
      (`ActorComponent.Deactivate` (`self.TailYawThrust`)))))

(event `InputAxis|EngineThrust`
  (params (AxisValue :type "Float (single-precision)"))
  ;[1 1 1] Handles Speed
  (`PrimitiveComponent.AddImpulse` (`self.ShipMesh`) (* (`KismetMathLibrary.GetForwardVector` (`SceneComponent.K2_GetComponentRotation` (`self.RootDirectionArrow`))) (* AxisValue (`self.EnginePower`))) "None" false))

(event `self.ReceiveBeginPlay`
  (bind _returnvalue (`PrimitiveComponent.CreateDynamicMaterialInstance` (`self.CylinderC`) 0 null))
  (set `self.MD_CylinderC` _returnvalue)
  (bind _returnvalue_2 (`PrimitiveComponent.CreateDynamicMaterialInstance` (`self.CylinderL`) 0 null))
  (set `self.MD_CylinderL` _returnvalue_2)
  (bind _returnvalue_3 (`PrimitiveComponent.CreateDynamicMaterialInstance` (`self.CylinderR`) 0 null))
  (set `self.MD_CylinderR` _returnvalue_3))

(event `self.ReceiveTick`
  (params (DeltaSeconds :type "Float (single-precision)"))
  (bind (_returnvalue_x _returnvalue_y _returnvalue_z) (`KismetMathLibrary.BreakVector` (`SceneComponent.GetComponentVelocity` (`self.ShipMesh`))))
  (bind _returnvalue (`KismetMathLibrary.LinearColorLerp` (struct :`R` 0.655 :`G` 0.655 :`B` 0.655 :`A` 1.0) (struct :`R` 1.0 :`G` 0.04934 :`B` 0.00954 :`A` 1.0) (`KismetMathLibrary.Abs` (/ (+ _returnvalue_x _returnvalue_y _returnvalue_z) 2500.0))))
  (`MaterialInstanceDynamic.SetVectorParameterValue` (`self.MD_CylinderL`) "thrust" _returnvalue)
  (`MaterialInstanceDynamic.SetVectorParameterValue` (`self.MD_CylinderR`) "thrust" _returnvalue)
  (`MaterialInstanceDynamic.SetVectorParameterValue` (`self.MD_CylinderC`) "thrust" _returnvalue))

(event `Key|LeftMouseButton`
  (params (Key :type "Key Structure" :default "AnyKey"))
  (bind _returnvalue (`KismetMathLibrary.MakeVector` (.x (`self.K2_GetActorLocation`)) (.y (`self.K2_GetActorLocation`)) (+ (.z (`self.K2_GetActorLocation`)) 60.0)))
  ;[1 1 1] Shooting
  (:`Pressed`
    (bind _outhit (`KismetSystemLibrary.LineTraceSingle` _returnvalue (+ (* (`SceneComponent.GetForwardVector` (`self.RootDirectionArrow`)) 100000.0) _returnvalue) "TraceTypeQuery1"))
    (bind (_bblockinghit _binitialoverlap _time _location _impactpoint _normal _impactnormal _physmat _hitactor) (`GameplayStatics.BreakHitResult` _outhit))
    (`GameplayStatics.SpawnEmitterAtLocation` "/Game/StarterContent/Particles/P_Explosion.P_Explosion" _location)
    (`GameplayStatics.PlaySoundAtLocation` "/Game/StarterContent/Audio/Explosion01.Explosion01" _location)
    (bind _asrock_84_blueprint (cast `/Game/Blueprints/Rock_84_Blueprint` _hitactor))
    (`/Game/Blueprints/Rock_84_Blueprint.DecreaseHealth` _asrock_84_blueprint)))

(fn `UserConstructionScript`)